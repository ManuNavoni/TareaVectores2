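; BP_Arquero is an archer Blueprint with the beginnings of logic for shooting arrows at one of two orcs.
; BeginPlay draws a long-lasting debug sphere around it, with a hard-coded radius.
; VerificarDistancia tests both orc distances against Alcance, and SetTarget compares them, but neither acts on the result.
; SpawnFlecha spawns BP_Flecha with a direction scaled by arrow speed; Tick is empty and nothing here calls these functions.
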(event `self.ReceiveBeginPlay`
  (`KismetSystemLibrary.DrawDebugSphere` (`self.K2_GetActorLocation`) 2000.0 36 (struct :`R` 0.098907 :`B` 1.0 :`A` 1.0) 3600.0 2.0))

(event `self.ReceiveTick`
  (params (DeltaSeconds :type "Float (single-precision)")))

(fn `SetTarget`
  (params (`Distancia Orco 1` :type "Float (double-precision)") (`Distancia Orco 2` :type "Float (double-precision)"))
  (if (>= (- `Distancia Orco 1` `Distancia Orco 2`) 0.0)
    _))

(fn `SpawnFlecha`
  (params (DireccionNormalizada :type "Vector Structure"))
  (bind _multip_velocidad_flecha (`self.Multip Velocidad Flecha`))
  (`|SpawnActorFromClass` "/Game/BluePrints/BP_Flecha.BP_Flecha_C" (`self.GetTransform`) "Undefined" "MultiplyWithRoot" null (`KismetMathLibrary.MakeVector` (* DireccionNormalizada_X _multip_velocidad_flecha) (* DireccionNormalizada_Y _multip_velocidad_flecha) (* DireccionNormalizada_Z _multip_velocidad_flecha)) null))

(fn `UserConstructionScript`)

(fn `VerificarDistancia`
  (params (`Distancia Orco 1` :type "Float (double-precision)") (`Distancia Orco 2` :type "Float (double-precision)"))
  (bind _alcance (`self.Alcance`))
  (if (<= `Distancia Orco 1` _alcance)
    (return)
    (elif (<= `Distancia Orco 2` _alcance)
      (return))))